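; Base component for DMX lighting fixture parts, providing helpers that turn DMX function values into visual changes.
; It can cache the owner's DMX component and store unique function names, leaving UpdateDMX as an empty event.
; Helpers map 8, 16 or 24-bit values onto material parameters, light color, intensity, spot cone, spring arm length and pan/tilt rotation.
; Color helpers add a fourth channel to RGB, capped at maximum.
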(event `self.ReceiveBeginPlay`)

(event `UpdateDMX`
  (params (dnDMXFunctions :type "Array of DMXAttributeName Structure") (NIMap_DMXFunctionValues :type "Map of DMXAttributeName Structure to Integer")))

(fn `InitDMXFunctionNames`
  (params (dnDMXFunctionNames :type "Array of DMXAttributeName Structure"))
  (bind _dndmxcomponentfunctions (`self.dnDMXComponentFunctions`))
  (`KismetArrayLibrary.Array_Clear` _dndmxcomponentfunctions)
  (for _array_element dnDMXFunctionNames
    (`KismetArrayLibrary.Array_AddUnique` _dndmxcomponentfunctions _array_element))
  (return))

(fn `SetParentDMXRef`
  (bind _returnvalue (`self.GetOwner`))
  (bind _returnvalue_2 (`Actor.GetComponentByClass` _returnvalue "/Script/DMXRuntime.DMXComponent"))
  (if (`KismetSystemLibrary.IsValid` _returnvalue_2)
    (set `self.DMXCompRef_ParentDMX` _returnvalue_2)
    (else
      (`KismetSystemLibrary.PrintString` (`KismetTextLibrary.Conv_TextToString` (`|FormatText` "Couldn't Find DMX Component on Parent Actor: {name}" (`KismetSystemLibrary.GetDisplayName` _returnvalue)))))))

(fn `UpdateDMXLightColor`
  (params (`DMX Parameter Bit Depth` :type "/Game/_Fixtures/_BlueprintComponents/E_DMXParamBitDepth Enum" :default "NewEnumerator0") (LightComponentRef :type "LightComponent Object Reference") (fRange :type "Float (double-precision)") (DIMap_DMXFunctionValues :type "Map of DMXAttributeName Structure to Integer") (dnDMXComponentFunctions :type "Array of DMXAttributeName Structure"))
  (locals (fMaxParameterRange :type Integer))
  (bind _returnvalue (`KismetMathLibrary.MapRangeClamped` (`KismetMathLibrary.Conv_IntToDouble` (`BlueprintMapLibrary.Map_Find` DIMap_DMXFunctionValues (`|GetArrayItem` dnDMXComponentFunctions 3))) 0.0 (`KismetMathLibrary.Conv_IntToDouble` (`local.fMaxParameterRange`)) 0.0 fRange))
  (`|ExecutionSequence`
    (:`then_0`
      (switch `/Game/_Fixtures/_BlueprintComponents/E_DMXParamBitDepth` `DMX Parameter Bit Depth`
        (:`NewEnumerator0`
          (set `local.fMaxParameterRange` 255))
        (:`NewEnumerator1`
          (set `local.fMaxParameterRange` 65535))
        (:`NewEnumerator2`
          (set `local.fMaxParameterRange` 16777215))))
    (:`then_1`
      (`LightComponent.SetLightColor` LightComponentRef (`KismetMathLibrary.MakeColor` (`KismetMathLibrary.FMin` (+ (`KismetMathLibrary.MapRangeClamped` (`KismetMathLibrary.Conv_IntToDouble` (`BlueprintMapLibrary.Map_Find` DIMap_DMXFunctionValues (`|GetArrayItem` dnDMXComponentFunctions))) 0.0 (`KismetMathLibrary.Conv_IntToDouble` (`local.fMaxParameterRange`)) 0.0 fRange) _returnvalue) fRange) (`KismetMathLibrary.FMin` (+ (`KismetMathLibrary.MapRangeClamped` (`KismetMathLibrary.Conv_IntToDouble` (`BlueprintMapLibrary.Map_Find` DIMap_DMXFunctionValues (`|GetArrayItem` dnDMXComponentFunctions 1))) 0.0 (`KismetMathLibrary.Conv_IntToDouble` (`local.fMaxParameterRange`)) 0.0 fRange) _returnvalue) fRange) (`KismetMathLibrary.FMin` (+ (`KismetMathLibrary.MapRangeClamped` (`KismetMathLibrary.Conv_IntToDouble` (`BlueprintMapLibrary.Map_Find` DIMap_DMXFunctionValues (`|GetArrayItem` dnDMXComponentFunctions 2))) 0.0 (`KismetMathLibrary.Conv_IntToDouble` (`local.fMaxParameterRange`)) 0.0 fRange) _returnvalue) fRange)) false))))

(fn `UpdateDMXLightIntensity`
  (params (`DMX Parameter Bit Depth` :type "/Game/_Fixtures/_BlueprintComponents/E_DMXParamBitDepth Enum" :default "NewEnumerator0") (LightComponentRef :type "LightComponent Object Reference") (fRange :type "Float (double-precision)") (DIMap_DMXFunctionValues :type "Map of DMXAttributeName Structure to Integer") (dnDMXComponentFunction :type "DMXAttributeName Structure"))
  (locals (fMaxParameterRange :type Integer))
  (`|ExecutionSequence`
    (:`then_0`
      (switch `/Game/_Fixtures/_BlueprintComponents/E_DMXParamBitDepth` `DMX Parameter Bit Depth`
        (:`NewEnumerator0`
          (set `local.fMaxParameterRange` 255))
        (:`NewEnumerator1`
          (set `local.fMaxParameterRange` 65535))
        (:`NewEnumerator2`
          (set `local.fMaxParameterRange` 16777215))))
    (:`then_1`
      (`LightComponent.SetIntensity` LightComponentRef (`KismetMathLibrary.MapRangeClamped` (`KismetMathLibrary.Conv_IntToDouble` (`BlueprintMapLibrary.Map_Find` DIMap_DMXFunctionValues dnDMXComponentFunction)) 0.0 (`KismetMathLibrary.Conv_IntToDouble` (`local.fMaxParameterRange`)) 0.0 fRange)))))

(fn `UpdateDMXMaterialScalarParameter`
  (params (miTargetMaterial :type "MaterialInstanceDynamic Object Reference") (`DMX Parameter Bit Depth` :type "/Game/_Fixtures/_BlueprintComponents/E_DMXParamBitDepth Enum" :default "NewEnumerator0") (nMaterialParameterName :type Name) (fScaleFactor :type "Float (double-precision)") (fRangeMin :type "Float (double-precision)") (fRangeMax :type "Float (double-precision)") (DIMap_DMXFunctionValues :type "Map of DMXAttributeName Structure to Integer") (dnDMXComponentFunction :type "DMXAttributeName Structure"))
  (locals (fMaxParameterRange :type Integer))
  (`|ExecutionSequence`
    (:`then_0`
      (switch `/Game/_Fixtures/_BlueprintComponents/E_DMXParamBitDepth` `DMX Parameter Bit Depth`
        (:`NewEnumerator0`
          (set `local.fMaxParameterRange` 255))
        (:`NewEnumerator1`
          (set `local.fMaxParameterRange` 65535))
        (:`NewEnumerator2`
          (set `local.fMaxParameterRange` 16777215))))
    (:`then_1`
      (`MaterialInstanceDynamic.SetScalarParameterValue` miTargetMaterial nMaterialParameterName (* (`KismetMathLibrary.MapRangeClamped` (`KismetMathLibrary.Conv_IntToDouble` (`BlueprintMapLibrary.Map_Find` DIMap_DMXFunctionValues dnDMXComponentFunction)) 0.0 (`KismetMathLibrary.Conv_IntToDouble` (`local.fMaxParameterRange`)) fRangeMin fRangeMax) fScaleFactor))
      (return))))

(fn `UpdateDMXMaterialVectorParameter`
  (params (miTargetMaterial :type "MaterialInstanceDynamic Object Reference") (`DMX Parameter Bit Depth` :type "/Game/_Fixtures/_BlueprintComponents/E_DMXParamBitDepth Enum" :default "NewEnumerator0") (nMaterialParameterName :type Name) (DIMap_DMXFunctionValues :type "Map of DMXAttributeName Structure to Integer") (dnDMXComponentFunctions :type "Array of DMXAttributeName Structure"))
  (locals (fMaxParameterRange :type Integer))
  (bind _returnvalue (`KismetMathLibrary.MapRangeClamped` (`KismetMathLibrary.Conv_IntToDouble` (`BlueprintMapLibrary.Map_Find` DIMap_DMXFunctionValues (`|GetArrayItem` dnDMXComponentFunctions 3))) 0.0 (`KismetMathLibrary.Conv_IntToDouble` (`local.fMaxParameterRange`)) 0.0 1.0))
  (`|ExecutionSequence`
    (:`then_0`
      (switch `/Game/_Fixtures/_BlueprintComponents/E_DMXParamBitDepth` `DMX Parameter Bit Depth`
        (:`NewEnumerator0`
          (set `local.fMaxParameterRange` 255))
        (:`NewEnumerator1`
          (set `local.fMaxParameterRange` 65535))
        (:`NewEnumerator2`
          (set `local.fMaxParameterRange` 16777215))))
    (:`then_1`
      (`MaterialInstanceDynamic.SetVectorParameterValue` miTargetMaterial nMaterialParameterName (make `LinearColor` (`KismetMathLibrary.FMin` (+ (`KismetMathLibrary.MapRangeClamped` (`KismetMathLibrary.Conv_IntToDouble` (`BlueprintMapLibrary.Map_Find` DIMap_DMXFunctionValues (`|GetArrayItem` dnDMXComponentFunctions))) 0.0 (`KismetMathLibrary.Conv_IntToDouble` (`local.fMaxParameterRange`)) 0.0 1.0) _returnvalue) 1.0) (`KismetMathLibrary.FMin` (+ (`KismetMathLibrary.MapRangeClamped` (`KismetMathLibrary.Conv_IntToDouble` (`BlueprintMapLibrary.Map_Find` DIMap_DMXFunctionValues (`|GetArrayItem` dnDMXComponentFunctions 1))) 0.0 (`KismetMathLibrary.Conv_IntToDouble` (`local.fMaxParameterRange`)) 0.0 1.0) _returnvalue) 1.0) (`KismetMathLibrary.FMin` (+ (`KismetMathLibrary.MapRangeClamped` (`KismetMathLibrary.Conv_IntToDouble` (`BlueprintMapLibrary.Map_Find` DIMap_DMXFunctionValues (`|GetArrayItem` dnDMXComponentFunctions 2))) 0.0 (`KismetMathLibrary.Conv_IntToDouble` (`local.fMaxParameterRange`)) 0.0 1.0) _returnvalue) 1.0) 1.0)))))

(fn `UpdateDMXRotation`
  (params (`DMX Parameter Bit Depth` :type "/Game/_Fixtures/_BlueprintComponents/E_DMXParamBitDepth Enum" :default "NewEnumerator0") (SceneComponentRef :type "SceneComponent Object Reference") (`Rotation Type` :type "/Game/_Fixtures/_BlueprintComponents/E_DMXRotationMode Enum" :default "NewEnumerator0") (fRange :type "Float (double-precision)") (DIMap_DMXFunctionValues :type "Map of DMXAttributeName Structure to Integer") (dnDMXComponentFunction :type "DMXAttributeName Structure"))
  (locals (fMaxParameterRange :type Integer))
  (bind _returnvalue (`KismetMathLibrary.MapRangeClamped` (`KismetMathLibrary.Conv_IntToDouble` (`BlueprintMapLibrary.Map_Find` DIMap_DMXFunctionValues dnDMXComponentFunction)) 0.0 (`KismetMathLibrary.Conv_IntToDouble` (`local.fMaxParameterRange`)) (* fRange -0.5) (* fRange 0.5)))
  (`|ExecutionSequence`
    (:`then_0`
      (switch `/Game/_Fixtures/_BlueprintComponents/E_DMXParamBitDepth` `DMX Parameter Bit Depth`
        (:`NewEnumerator0`
          (set `local.fMaxParameterRange` 255))
        (:`NewEnumerator1`
          (set `local.fMaxParameterRange` 65535))
        (:`NewEnumerator2`
          (set `local.fMaxParameterRange` 16777215))))
    (:`then_1`
      (switch `/Game/_Fixtures/_BlueprintComponents/E_DMXRotationMode` `Rotation Type`
        (:`NewEnumerator0`
          (`SceneComponent.K2_SetRelativeRotation` SceneComponentRef (`KismetMathLibrary.MakeRotator` 0.0 0.0 _returnvalue) false false))
        (:`NewEnumerator1`
          (`SceneComponent.K2_SetRelativeRotation` SceneComponentRef (`KismetMathLibrary.MakeRotator` _returnvalue) false false))))))

(fn `UpdateDMXSpotConeAngle`
  (params (`DMX Parameter Bit Depth` :type "/Game/_Fixtures/_BlueprintComponents/E_DMXParamBitDepth Enum" :default "NewEnumerator0") (LightComponentRef :type "LightComponent Object Reference") (fBeamRangeMax :type "Float (double-precision)") (fBeamRangeMin :type "Float (double-precision)") (DIMap_DMXFunctionValues :type "Map of DMXAttributeName Structure to Integer") (dnDMXComponentFunction :type "DMXAttributeName Structure"))
  (locals (fMaxParameterRange :type Integer))
  (bind _returnvalue (* (`KismetMathLibrary.MapRangeClamped` (`KismetMathLibrary.Conv_IntToDouble` (`BlueprintMapLibrary.Map_Find` DIMap_DMXFunctionValues dnDMXComponentFunction)) 0.0 (`KismetMathLibrary.Conv_IntToDouble` (`local.fMaxParameterRange`)) fBeamRangeMax fBeamRangeMin) 0.7))
  (`|ExecutionSequence`
    (:`then_0`
      (switch `/Game/_Fixtures/_BlueprintComponents/E_DMXParamBitDepth` `DMX Parameter Bit Depth`
        (:`NewEnumerator0`
          (set `local.fMaxParameterRange` 255))
        (:`NewEnumerator1`
          (set `local.fMaxParameterRange` 65535))
        (:`NewEnumerator2`
          (set `local.fMaxParameterRange` 16777215))))
    (:`then_1`
      (bind _asspot_light_component (cast `SpotLightComponent` LightComponentRef))
      (`SpotLightComponent.SetOuterConeAngle` _asspot_light_component _returnvalue)
      (`SpotLightComponent.SetInnerConeAngle` _asspot_light_component (* _returnvalue 0.7))
      (return))))

(fn `UpdateDMXSpringArm`
  (params (`DMX Parameter Bit Depth` :type "/Game/_Fixtures/_BlueprintComponents/E_DMXParamBitDepth Enum" :default "NewEnumerator0") (SpringArmComponentRef :type "SpringArmComponent Object Reference") (fRange :type "Float (double-precision)") (DIMap_DMXFunctionValues :type "Map of DMXAttributeName Structure to Integer") (nDMXComponentFunction :type "DMXAttributeName Structure"))
  (locals (fMaxParameterRange :type Integer))
  (`|ExecutionSequence`
    (:`then_0`
      (switch `/Game/_Fixtures/_BlueprintComponents/E_DMXParamBitDepth` `DMX Parameter Bit Depth`
        (:`NewEnumerator0`
          (set `local.fMaxParameterRange` 255))
        (:`NewEnumerator1`
          (set `local.fMaxParameterRange` 65535))
        (:`NewEnumerator2`
          (set `local.fMaxParameterRange` 16777215))))
    (:`then_1`
      (set `SpringArmComponent.TargetArmLength` (`KismetMathLibrary.MapRangeClamped` (`KismetMathLibrary.Conv_IntToDouble` (`BlueprintMapLibrary.Map_Find` DIMap_DMXFunctionValues nDMXComponentFunction)) 0.0 (`KismetMathLibrary.Conv_IntToDouble` (`local.fMaxParameterRange`)) 0.0 fRange) SpringArmComponentRef)
      (return))))
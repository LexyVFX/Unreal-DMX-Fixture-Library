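; BP_Impression_FR1 is the DMX lighting fixture actor for the GLP Impression FR1.
; On BeginPlay it binds to the DMX subsystem's protocol-received event and gathers unique function definitions from its BP_DMXBaseComponent components.
; Each received event reads the active-mode function values from the fixture patch, then passes them with those definitions to every such component to update.
; A BeginPlay loop over static mesh material slots has no effect.
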(event `self.ReceiveBeginPlay`
  (`|ExecutionSequence`
    (:`then_0`
      (add `DMXSubsystem.OnProtocolReceived` (subsystem `DMXSubsystem`) (delegate `Received DMX`))
      (`self.InitDMXFunctionNames`))
    (:`then_1`
      (for _array_element (`self.K2_GetComponentsByClass` "/Script/Engine.StaticMeshComponent")
        (`/Engine/EditorBlueprintResources/StandardMacros.IsValid` _array_element
          (:`Is Valid`
            (for _ (`MeshComponent.GetMaterialSlotNames` _array_element)
              _)))))))

(event `Received DMX`
  (params (Protocol :type "DMXProtocolName Structure") (Universe :type Integer) (DMXBuffer :type "Array of Byte (by ref)"))
  (bind _outfunctionsmap (`self.GetDMXFunctionValues` Protocol))
  (`self.UpdateDMXComponents` _outfunctionsmap))

(fn `GetDMXFunctionValues`
  (params (eDmxType :type "DMXProtocolName Structure"))
  (returns (OutFunctionsMap :type "Map of Name to Integer"))
  (bind _returnvalue (`DMXComponent.GetFixturePatch` (`self.DMX`)))
  (`/Engine/EditorBlueprintResources/StandardMacros.IsValid` _returnvalue
    (:`Is Valid`
      (bind _outfunctionsmap (`|GetDMXActiveModeFunctionValues` _returnvalue eDmxType))
      (return _outfunctionsmap))))

(fn `InitDMXFunctionNames`
  (`KismetArrayLibrary.Array_Clear` (`self.sDMXFunctions`))
  (for _array_element (`self.K2_GetComponentsByClass` "/Game/_Fixtures/_BlueprintComponents/BP_DMXBaseComponent.BP_DMXBaseComponent_C")
    (`/Engine/EditorBlueprintResources/StandardMacros.IsValid` _array_element
      (:`Is Valid`
        (`KismetArrayLibrary.Array_AddUnique` (`self.sDMXFunctions`) (`/Game/_Fixtures/_BlueprintComponents/BP_DMXBaseComponent.sDMXComponentFunctions` _array_element))))))

(fn `UpdateDMXComponents`
  (params (niMap_DMXFunctionValues :type "Map of Name to Integer"))
  (bind _returnvalue (`self.K2_GetComponentsByClass` "/Game/_Fixtures/_BlueprintComponents/BP_DMXBaseComponent.BP_DMXBaseComponent_C"))
  (bind _output_get (set `self.niMap_DMXFunctionValues` niMap_DMXFunctionValues))
  (for _ _returnvalue
    (`/Game/_Fixtures/_BlueprintComponents/BP_DMXBaseComponent.UpdateDMX` _returnvalue (`self.sDMXFunctions`) _output_get)))

(fn `UserConstructionScript`)
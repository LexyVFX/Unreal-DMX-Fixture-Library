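; DMX fixture component that drives the tilt rotation of the owning actor's head mesh from incoming DMX values.
; On BeginPlay it sets its parent DMX reference, initializes its DMX function names, and caches the first static mesh component whose display name contains "Head".
; Each UpdateDMX event passes the function values, bit depth and range to UpdateDMXRotation to rotate that mesh.
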(event `self.ReceiveBeginPlay`
  (`|ExecutionSequence`
    (:`then_0`
      (`self.SetParentDMXRef`))
    (:`then_1`
      (`self.InitDMXFunctionNames` (`|MakeArray` (struct :`Name` "Tilt") :!type "DMXAttributeName Structure")))
    (:`then_2`
      (for _array_element (`Actor.K2_GetComponentsByClass` (`self.GetOwner`) "/Script/Engine.StaticMeshComponent")
        (if (`KismetStringLibrary.Contains` (`KismetSystemLibrary.GetDisplayName` _array_element) "Head")
          (set `self.SMRef_Head` _array_element)
          (break))))))

(event `self.UpdateDMX`
  (params (dnDMXFunctions :type "Array of DMXAttributeName Structure (by ref)") (NIMap_DMXFunctionValues :type "Map of DMXAttributeName Structure to Integer"))
  (`self.UpdateDMXRotation` (`self.E_DMXParamaterBitDepth`) (`self.SMRef_Head`) "NewEnumerator1" (`self.fRange`) NIMap_DMXFunctionValues (struct :`Name` "Tilt")))
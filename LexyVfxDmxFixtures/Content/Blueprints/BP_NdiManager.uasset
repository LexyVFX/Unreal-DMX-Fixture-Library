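; BP_NdiManager connects its NDI receiver components to named network video streams.
; On begin play and whenever network sources change, it pairs receivers with stream entries by index, moving the Resolume receiver out of first place.
; IntializeNDI finds each idle entry's source by name, starts the receiver and broadcasts the source change.
; Pressing Enter shuts down all receivers, resets their entries and reconnects.
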(event `self.ReceiveBeginPlay`
  (`self.Event On Find Network Connection and Stream` :!label _label))

(event `Key|Enter`
  (params (Key :type "Key Structure"))
  (bind _struct_ndiinputs (`self.Struct_NdiInputs`))
  (:`Pressed`
    (for (_array_element _array_index) (`self.K2_GetComponentsByClass` "/Script/NDIIO.NDIReceiverComponent")
      (`NDIReceiverComponent.ShutdownReceiver` _array_element)
      (bind (_output_bcurrentlyreceiving _output_str_streamname _output_ci_currentconnection) (break `/Game/Blueprints/Struct_NdiInput` (`|GetArrayItem` _struct_ndiinputs _array_index)))
      (`KismetArrayLibrary.Array_Set` _struct_ndiinputs _array_index (make `/Game/Blueprints/Struct_NdiInput` false _output_str_streamname _output_ci_currentconnection)))
    (goto _label)))

(event `self.NDIFinderComponent.OnNetworkSourcesChanged`
  (params (InComponent :type "NDIFinderComponent Object Reference"))
  (`self.Event On Find Network Connection and Stream`))

(event `Event On Find Network Connection and Stream`
  (bind _output_get (set `self.tempNdiReceivers` (`self.K2_GetComponentsByClass` "/Script/NDIIO.NDIReceiverComponent")))
  (if (== (`KismetArrayLibrary.Array_Find` _output_get (`self.NDIReceiverComponent_Resolume`)) 0)
    (`KismetArrayLibrary.Array_Swap` _output_get 1))
  (for (_array_element _array_index) _output_get
    (`self.IntializeNDI` (`|GetArrayItem` (`self.Struct_NdiInputs`) _array_index) _array_element _array_index)
    (`KismetSystemLibrary.PrintString` (`KismetTextLibrary.Conv_TextToString` (`|FormatText` "{id}:{name}" _array_index (`KismetSystemLibrary.GetDisplayName` _array_element))))))

(fn `IntializeNDI`
  (params (`NDI Input Info` :type "/Game/Blueprints/Struct_NdiInput Structure (by ref)") (ReceiverComponent :type "NDIReceiverComponent Object Reference (by ref)") (ComponentIndex :type Integer))
  (bind (_bcurrentlyreceiving _str_streamname) (break `/Game/Blueprints/Struct_NdiInput` `NDI Input Info`))
  (bind _struct_ndiinputs (`self.Struct_NdiInputs`))
  (bind (_output_bcurrentlyreceiving _output_str_streamname) (break `/Game/Blueprints/Struct_NdiInput` (`|GetArrayItem` _struct_ndiinputs ComponentIndex)))
  (if (not _bcurrentlyreceiving)
    (bind (_connectioninformation _returnvalue) (`NDIFinderComponent.FindNetworkSourceByName` (`self.NDIFinderComponent`) _str_streamname))
    (`KismetArrayLibrary.Array_Set` _struct_ndiinputs ComponentIndex (make `/Game/Blueprints/Struct_NdiInput` _output_bcurrentlyreceiving _output_str_streamname _connectioninformation))
    (if _returnvalue
      (`KismetArrayLibrary.Array_Set` _struct_ndiinputs ComponentIndex (make `/Game/Blueprints/Struct_NdiInput` true _output_str_streamname _connectioninformation))
      (`NDIReceiverComponent.StartReceiver` ReceiverComponent _connectioninformation)
      (`NDIReceiverComponent.ChangeConnection` ReceiverComponent _connectioninformation)
      (`self.Change Network Source Connection` (`KismetTextLibrary.Conv_StringToText` (`.SourceName` (break `NDIConnectionInformation` _connectioninformation)))) ; Remote Bindable Delegate for making other actors aware of source changes
    )))

(fn `UserConstructionScript`)
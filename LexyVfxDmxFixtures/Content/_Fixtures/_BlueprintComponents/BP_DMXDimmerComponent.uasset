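; DMX fixture component that drives the dimmer of a stage light from incoming DMX values.
; On BeginPlay it registers the "Dimmer" function, caches the owner's spotlight and finds beam and lens meshes by name to create dynamic materials.
; UpdateDMX remaps the 8-bit or 16-bit value to a normalized "DMX Dimmer" parameter on both materials and to the spotlight's intensity, scaled by a configurable maximum.
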(event `self.ReceiveBeginPlay`
  (bind _smref_beam (`self.SMRef_Beam`))
  (bind _smref_lens (`self.SMRef_Lens`))
  (bind _returnvalue (`Actor.GetComponentByClass` (`self.GetOwner`) "/Script/Engine.SpotLightComponent"))
  (`|ExecutionSequence`
    (:`then_0`
      (`self.SetParentDMXRef`))
    (:`then_1`
      (`self.InitDMXFunctionNames` (`|MakeArray` "Dimmer" :!type "Name")))
    (:`then_2`
      (`/Engine/EditorBlueprintResources/StandardMacros.IsValid` _returnvalue
        (:`Is Valid`
          (set `self.SpotRef_Light` _returnvalue))))
    (:`then_3`
      (for _array_element (`Actor.K2_GetComponentsByClass` (`self.GetOwner`) "/Script/Engine.StaticMeshComponent")
        (`|ExecutionSequence`
          (:`then_0`
            (bind _returnvalue_2 (`KismetSystemLibrary.GetDisplayName` _array_element))
            (if (`KismetStringLibrary.Contains` _returnvalue_2 "Beam")
              (set `self.SMRef_Beam` _array_element)))
          (:`then_1`
            (if (`KismetStringLibrary.Contains` _returnvalue_2 "Lens")
              (set `self.SMRef_Lens` _array_element)))))
      (`|ExecutionSequence`
        (:`then_0`
          (bind _returnvalue_3 (`PrimitiveComponent.CreateDynamicMaterialInstance` _smref_beam 0 (`PrimitiveComponent.GetMaterial` _smref_beam 0) "None"))
          (set `self.miBeam` _returnvalue_3))
        (:`then_1`
          (bind _returnvalue_4 (`PrimitiveComponent.CreateDynamicMaterialInstance` _smref_lens 0 (`PrimitiveComponent.GetMaterial` _smref_lens 0) "None"))
          (set `self.miLens` _returnvalue_4))))))

(event `self.UpdateDMX`
  (params (sDMXFunctions :type "Array of /Game/_Fixtures/_BlueprintComponents/S_DMXComponentFunctions Structure (by ref)") (NIMap_DMXFunctionValues :type "Map of Name to Integer"))
  (bind _sdmxcomponentfunctions_ndmxcomponentfunctions (break `/Game/_Fixtures/_BlueprintComponents/S_DMXComponentFunctions` (`self.sDMXComponentFunctions`)))
  (bind _milens (`self.miLens`))
  (bind _mibeam (`self.miBeam`))
  (bind _spotref_light (`self.SpotRef_Light`))
  (bind _flightintensity (`self.fLightIntensity`))
  (bind _value (`BlueprintMapLibrary.Map_Find` NIMap_DMXFunctionValues (`|GetArrayItem` _sdmxcomponentfunctions_ndmxcomponentfunctions)))
  (bind _returnvalue (`KismetMathLibrary.Conv_IntToDouble` _value))
  (bind _returnvalue_2 (`KismetMathLibrary.Conv_IntToDouble` _value))
  (bind _returnvalue_3 (`KismetMathLibrary.MapRangeClamped` _returnvalue_2 0.0 255.0 0.0 1.0))
  (bind _returnvalue_4 (`KismetMathLibrary.MapRangeClamped` _returnvalue_2 0.0 65535.0 0.0 1.0))
  (if (`self.b16Bit`)
    (`MaterialInstanceDynamic.SetScalarParameterValue` _mibeam "DMX Dimmer" _returnvalue_4)
    (`MaterialInstanceDynamic.SetScalarParameterValue` _milens "DMX Dimmer" _returnvalue_4)
    (`LightComponent.SetIntensity` _spotref_light (`KismetMathLibrary.MapRangeClamped` _returnvalue 0.0 65535.0 0.0 _flightintensity))
    (else
      (`MaterialInstanceDynamic.SetScalarParameterValue` _mibeam "DMX Dimmer" _returnvalue_3)
      (`MaterialInstanceDynamic.SetScalarParameterValue` _milens "DMX Dimmer" _returnvalue_3)
      (`LightComponent.SetIntensity` _spotref_light (`KismetMathLibrary.MapRangeClamped` _returnvalue 0.0 255.0 0.0 _flightintensity)))))
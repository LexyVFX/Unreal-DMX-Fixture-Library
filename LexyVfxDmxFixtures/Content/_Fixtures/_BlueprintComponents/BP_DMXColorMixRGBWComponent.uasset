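; DMX fixture component that applies four-channel color mixing (RGBW, per its name) to the owning actor's light, beam and lens.
; On BeginPlay it sets the parent DMX reference and function names, finds the SpotLight and the "Beam" and "Lens" meshes by display name, and creates dynamic materials for both meshes.
; UpdateDMX converts incoming function values into the "DMX Color" parameter on both materials and the spotlight's color.
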(event `self.ReceiveBeginPlay`
  (bind _smref_beam (`self.SMRef_Beam`))
  (bind _smref_lens (`self.SMRef_Lens`))
  (bind _returnvalue (`Actor.GetComponentByClass` (`self.GetOwner`) "/Script/Engine.SpotLightComponent"))
  (`|ExecutionSequence`
    (:`then_0`
      (`self.SetParentDMXRef`))
    (:`then_1`
      (`self.InitDMXFunctionNames` (`|MakeArray` (struct :`Name` "Red") (struct :`Name` "Green") (struct :`Name` "Blue") (struct :`Name` "White") :!type "DMXAttributeName Structure")))
    (:`then_2`
      (`/Engine/EditorBlueprintResources/StandardMacros.IsValid` _returnvalue
        (:`Is Valid`
          (set `self.SpotRef_Light` _returnvalue))))
    (:`then_3`
      (for _array_element (`Actor.K2_GetComponentsByClass` (`self.GetOwner`) "/Script/Engine.StaticMeshComponent")
        (`|ExecutionSequence`
          (:`then_0`
            (bind _returnvalue_2 (`KismetSystemLibrary.GetDisplayName` _array_element))
            (if (`KismetStringLibrary.Contains` _returnvalue_2 "Beam")
              (set `self.SMRef_Beam` _array_element)))
          (:`then_1`
            (if (`KismetStringLibrary.Contains` _returnvalue_2 "Lens")
              (set `self.SMRef_Lens` _array_element)))))
      (`|ExecutionSequence`
        (:`then_0`
          (bind _returnvalue_3 (`PrimitiveComponent.CreateDynamicMaterialInstance` _smref_beam 0 (`PrimitiveComponent.GetMaterial` _smref_beam 0) "None"))
          (set `self.miBeam` _returnvalue_3))
        (:`then_1`
          (bind _returnvalue_4 (`PrimitiveComponent.CreateDynamicMaterialInstance` _smref_lens 0 (`PrimitiveComponent.GetMaterial` _smref_lens 0) "None"))
          (set `self.miLens` _returnvalue_4))))))

(event `self.UpdateDMX`
  (params (dnDMXFunctions :type "Array of DMXAttributeName Structure (by ref)") (NIMap_DMXFunctionValues :type "Map of DMXAttributeName Structure to Integer"))
  (bind _array (`|MakeArray` (struct :`Name` "Red") (struct :`Name` "Green") (struct :`Name` "Blue") (struct :`Name` "White") :!type "DMXAttributeName Structure"))
  (`self.UpdateDMXMaterialVectorParameter` (`self.miBeam`) (`self.E_DMXParamaterBitDepth`) "DMX Color" NIMap_DMXFunctionValues _array)
  (`self.UpdateDMXMaterialVectorParameter` (`self.miLens`) (`self.E_DMXParamaterBitDepth`) "DMX Color" NIMap_DMXFunctionValues _array)
  (`self.UpdateDMXLightColor` (`self.E_DMXParamaterBitDepth`) (`self.SpotRef_Light`) 1.0 NIMap_DMXFunctionValues _array))
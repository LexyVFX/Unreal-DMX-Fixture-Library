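; DMX fixture component that applies the Zoom channel to the owning light fixture's lens and beam.
; On BeginPlay it registers the Zoom function, caches the owner's spring arm and spot light, and creates a dynamic material on the mesh named "Beam".
; Each DMX update feeds that value to the spring arm, the beam material's zoom parameter (scaled, with range ends swapped) and the spot cone angle.
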(event `self.ReceiveBeginPlay`
  (bind _smref_beam (`self.SMRef_Beam`))
  (bind _returnvalue (`Actor.GetComponentByClass` (`self.GetOwner`) "/Script/Engine.SpringArmComponent"))
  (bind _returnvalue_2 (`Actor.GetComponentByClass` (`self.GetOwner`) "/Script/Engine.SpotLightComponent"))
  (`|ExecutionSequence`
    (:`then_0`
      (`self.SetParentDMXRef`))
    (:`then_1`
      (`self.InitDMXFunctionNames` (`|MakeArray` "Zoom" :!type "Name")))
    (:`then_2`
      (`/Engine/EditorBlueprintResources/StandardMacros.IsValid` _returnvalue
        (:`Is Valid`
          (set `self.SpRef_LensSpringArm` _returnvalue))))
    (:`then_3`
      (`/Engine/EditorBlueprintResources/StandardMacros.IsValid` _returnvalue_2
        (:`Is Valid`
          (set `self.SpotRef_Light` _returnvalue_2))))
    (:`then_4`
      (for _array_element (`Actor.K2_GetComponentsByClass` (`self.GetOwner`) "/Script/Engine.StaticMeshComponent")
        (if (`KismetStringLibrary.Contains` (`KismetSystemLibrary.GetDisplayName` _array_element) "Beam")
          (set `self.SMRef_Beam` _array_element)
          (break)))
      (bind _returnvalue_3 (`PrimitiveComponent.CreateDynamicMaterialInstance` _smref_beam 0 (`PrimitiveComponent.GetMaterial` _smref_beam 0) "None"))
      (set `self.miBeam` _returnvalue_3))))

(event `self.UpdateDMX`
  (params (sDMXFunctions :type "Array of /Game/_Fixtures/_BlueprintComponents/S_DMXComponentFunctions Structure (by ref)") (NIMap_DMXFunctionValues :type "Map of Name to Integer"))
  (bind _sdmxcomponentfunctions_ndmxcomponentfunctions (break `/Game/_Fixtures/_BlueprintComponents/S_DMXComponentFunctions` (`self.sDMXComponentFunctions`)))
  (bind _output (`|GetArrayItem` _sdmxcomponentfunctions_ndmxcomponentfunctions))
  (`self.UpdateDMXSpringArm` (`self.E_DMXParamaterBitDepth`) (`self.SpRef_LensSpringArm`) (`self.fBeamRangeLinear`) NIMap_DMXFunctionValues _output)
  (`self.UpdateDMXMaterialScalarParameter` (`self.miBeam`) (`self.E_DMXParamaterBitDepth`) "DMX Zoom" 1.3 (`self.fBeamRangeMax`) (`self.fBeamRangeMin`) NIMap_DMXFunctionValues _output)
  (`self.UpdateDMXSpotConeAngle` (`self.E_DMXParamaterBitDepth`) (`self.SpotRef_Light`) (`self.fBeamRangeMax`) (`self.fBeamRangeMin`) NIMap_DMXFunctionValues _output))
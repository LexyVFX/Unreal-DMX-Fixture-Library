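; BP_DMXPanComponent is a DMX fixture component that drives the pan rotation of a moving-head fixture's yoke.
; On BeginPlay it sets its parent DMX reference, registers the "Pan" function, and finds the owner's static mesh whose name contains "Yoke".
; UpdateDMX maps the 8-bit or 16-bit Pan value onto a range centered on zero, sized by FRange, and applies it as the yoke's relative yaw.
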(event `self.ReceiveBeginPlay`
  (`|ExecutionSequence`
    (:`then_0`
      (`self.SetParentDMXRef`))
    (:`then_1`
      (`self.InitDMXFunctionNames` (`|MakeArray` "Pan" :!type "Name")))
    (:`then_2`
      (for _array_element (`Actor.K2_GetComponentsByClass` (`self.GetOwner`) "/Script/Engine.StaticMeshComponent")
        (if (`KismetStringLibrary.Contains` (`KismetSystemLibrary.GetDisplayName` _array_element) "Yoke")
          (set `self.SMRef_Yoke` _array_element)
          (break))))))

(event `self.UpdateDMX`
  (params (sDMXFunctions :type "Array of /Game/_Fixtures/_BlueprintComponents/S_DMXComponentFunctions Structure (by ref)") (NIMap_DMXFunctionValues :type "Map of Name to Integer"))
  (bind _sdmxcomponentfunctions_ndmxcomponentfunctions (break `/Game/_Fixtures/_BlueprintComponents/S_DMXComponentFunctions` (`self.sDMXComponentFunctions`)))
  (bind _smref_yoke (`self.SMRef_Yoke`))
  (bind _frange (`self.fRange`))
  (bind _returnvalue (* _frange 0.5))
  (bind _returnvalue_2 (* _frange -0.5))
  (bind _returnvalue_3 (`KismetMathLibrary.Conv_IntToDouble` (`BlueprintMapLibrary.Map_Find` NIMap_DMXFunctionValues (`|GetArrayItem` _sdmxcomponentfunctions_ndmxcomponentfunctions))))
  (if (`self.b16Bit`)
    (`SceneComponent.K2_SetRelativeRotation` _smref_yoke (`KismetMathLibrary.MakeRotator` 0.0 0.0 (`KismetMathLibrary.MapRangeClamped` _returnvalue_3 0.0 65535.0 _returnvalue_2 _returnvalue)) false false)
    (else
      (`SceneComponent.K2_SetRelativeRotation` _smref_yoke (`KismetMathLibrary.MakeRotator` 0.0 0.0 (`KismetMathLibrary.MapRangeClamped` _returnvalue_3 0.0 255.0 _returnvalue_2 _returnvalue)) false false))))